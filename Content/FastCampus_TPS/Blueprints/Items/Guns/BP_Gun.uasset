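; BP_Gun is a gun item that a player can pick up by interacting with it.
; On interaction it passes itself to the player's PickUp, then sets its weapon state to Pickuped.
; SetWeaponState stores the state and switches the Sphere's collision profile, overlapping all dynamic objects when Dropped and disabling collision when Pickuped.
; The file contains no firing logic, and its default event nodes are disabled.
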(event `/Game/FastCampus_TPS/Blueprints/Items/BPI_Interaction.OnInteracted`
  (params (InPlayer :type "/Game/FastCampus_TPS/Blueprints/BP_Player_Character Object Reference"))
  (`/Game/FastCampus_TPS/Blueprints/BP_Player_Character.PickUp` InPlayer self)
  (`self.SetWeaponState` "NewEnumerator1"))

(fn `SetWeaponState`
  (params (NewState :type "/Game/FastCampus_TPS/Blueprints/Items/Guns/EWeaponState Enum" :default "NewEnumerator0"))
  (bind _output_get (set `self.WeaponState` NewState))
  (switch `/Game/FastCampus_TPS/Blueprints/Items/Guns/EWeaponState` _output_get
    (:`NewEnumerator0`
      (`PrimitiveComponent.SetCollisionProfileName` (`self.Sphere`) "OverlapAllDynamic" true))
    (:`NewEnumerator1`
      (`PrimitiveComponent.SetCollisionProfileName` (`self.Sphere`) "NoCollision" true))))

(fn `UserConstructionScript`
  (`parent.UserConstructionScript`))