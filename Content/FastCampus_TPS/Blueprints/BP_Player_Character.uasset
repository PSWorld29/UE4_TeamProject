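; Third-person shooter player character with camera-relative movement, walk/run speeds, hold-to-aim and two weapon slots.
; Aiming locks yaw to the controller, notifies the AnimBP and HUD reticle, and moves the camera between relaxed and ADS booms.
; Capsule overlaps and the Interaction input message actors through BPI_Interaction.
; PickUp fills the primary then secondary slot, using slot checks to attach weapons to hand or holster sockets.
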(event `self.ReceiveBeginPlay`
  (set `self.ABP_Player_Character` (`SkeletalMeshComponent.GetAnimInstance` (`self.Mesh`)))
  (message `/Game/FastCampus_TPS/Blueprints/Animations/BPI_Character_Animation.SetAimOffset` (`self.ABP_Player_Character`) (`self.StandAimOffset`)))

(event `InputAxis|Turn`
  (params (AxisValue :type "Float (single-precision)"))
  (`self.AddControllerYawInput` AxisValue))

(event `InputAxis|LookUp`
  (params (AxisValue :type "Float (single-precision)"))
  (`self.AddControllerPitchInput` AxisValue))

(event `InputAxis|MoveForward`
  (params (AxisValue :type "Float (single-precision)"))
  (bind (_returnvalue_roll _returnvalue_pitch _returnvalue_yaw) (`KismetMathLibrary.BreakRotator` (`self.GetControlRotation`)))
  (`self.AddMovementInput` (`KismetMathLibrary.GetForwardVector` (`KismetMathLibrary.MakeRotator` 0.0 0.0 _returnvalue_yaw)) AxisValue))

(event `InputAxis|MoveRight`
  (params (AxisValue :type "Float (single-precision)"))
  (bind (_returnvalue_roll _returnvalue_pitch _returnvalue_yaw) (`KismetMathLibrary.BreakRotator` (`self.GetControlRotation`)))
  (`self.AddMovementInput` (`KismetMathLibrary.GetRightVector` (`KismetMathLibrary.MakeRotator` 0.0 0.0 _returnvalue_yaw)) AxisValue))

(event `InputAction|Walk`
  (params (Key :type "Key Structure"))
  (bind _charactermovement (`self.CharacterMovement`))
  (:`Pressed`
    (set `CharacterMovementComponent.MaxWalkSpeed` (`self.WalkSpeed`) _charactermovement))
  (:`Released`
    (set `CharacterMovementComponent.MaxWalkSpeed` (`self.RunSpeed`) _charactermovement)))

(event `/Game/FastCampus_TPS/Blueprints/BPI_Chracter.AimDown`
  (params (AimEnable :type Boolean))
  (bind _output_get (set `self.bIsAimDown` AimEnable))
  (set `self.bUseControllerRotationYaw` _output_get)
  (message `/Game/FastCampus_TPS/Blueprints/Animations/BPI_Character_Animation.EnableAim` (`self.ABP_Player_Character`) _output_get)
  (message `/Game/FastCampus_TPS/Blueprints/UIs/BPI_UserInterface.EnableReticle` (`PlayerController.GetHUD` (`GameplayStatics.GetPlayerController` 0)) _output_get))

(event `InputAction|ToggleAim`
  (params (Key :type "Key Structure"))
  (:`Pressed`
    (`/Game/FastCampus_TPS/Blueprints/BPI_Chracter.AimDown` true)
    (`SceneComponent.K2_AttachToComponent` (`self.Camera`) (select `bool` (`self.bIsAimDown`) :`false` (`self.Camera Boom_Stand_rlx`) :`true` (`self.Camera Boom_Stand_ADS`) :!type "SceneComponent Object Reference") "None" "KeepWorld" "KeepWorld" "KeepWorld" true :!label _label)
    (`KismetSystemLibrary.MoveComponentTo` (`self.Camera`) (0.0 0.0 0.0) (struct) false false 0.2 true))
  (:`Released`
    (`/Game/FastCampus_TPS/Blueprints/BPI_Chracter.AimDown` false)
    (goto _label)))

(event `self.CapsuleComponent.OnComponentBeginOverlap`
  (params (OverlappedComponent :type "PrimitiveComponent Object Reference") (OtherActor :type "Actor Object Reference") (OtherComp :type "PrimitiveComponent Object Reference") (OtherBodyIndex :type Integer) (bFromSweep :type Boolean) (SweepResult :type "HitResult Structure (by ref)"))
  (if (`KismetSystemLibrary.DoesImplementInterface` OtherActor "/Game/FastCampus_TPS/Blueprints/Items/BPI_Interaction.BPI_Interaction_C")
    (message `/Game/FastCampus_TPS/Blueprints/Items/BPI_Interaction.OnInteractionRangeEntered` OtherActor self)))

(event `self.CapsuleComponent.OnComponentEndOverlap`
  (params (OverlappedComponent :type "PrimitiveComponent Object Reference") (OtherActor :type "Actor Object Reference") (OtherComp :type "PrimitiveComponent Object Reference") (OtherBodyIndex :type Integer))
  (if (`KismetSystemLibrary.DoesImplementInterface` OtherActor "/Game/FastCampus_TPS/Blueprints/Items/BPI_Interaction.BPI_Interaction_C")
    (message `/Game/FastCampus_TPS/Blueprints/Items/BPI_Interaction.OnInteractionRangeExited` OtherActor)))

(event `InputAction|Interaction`
  (params (Key :type "Key Structure"))
  (:`Pressed`
    (for _array_element (`PrimitiveComponent.GetOverlappingActors` (`self.CapsuleComponent`) "/Script/Engine.Actor")
      (if (`KismetSystemLibrary.DoesImplementInterface` _array_element "/Game/FastCampus_TPS/Blueprints/Items/BPI_Interaction.BPI_Interaction_C")
        (message `/Game/FastCampus_TPS/Blueprints/Items/BPI_Interaction.OnInteracted` _array_element self)))))

(fn `EquipWeapon`
  (params (Weapon :type "/Game/FastCampus_TPS/Blueprints/Items/Guns/BP_Gun Object Reference"))
  (`self.K2_AttachToComponent` Weapon (`self.Mesh`) "hand_rSocket" "SnapToTarget" "SnapToTarget" "SnapToTarget" true))

(fn `GetWeaponSocket`
  (params (SocketName :type Name))
  (returns (SocketTransform :type "Transform Structure"))
  (bind _weapon (`self.Weapon`))
  (`/Engine/EditorBlueprintResources/StandardMacros.IsValid` _weapon
    (:`Is Valid`
      (return (`SceneComponent.GetSocketTransform` _weapon SocketName "RTS_World")))))

(fn `PickUp`
  (params (Weapon :type "/Game/FastCampus_TPS/Blueprints/Items/Guns/BP_Gun Object Reference"))
  (`self.PrimaryWeapon`
    (:`then`
      (`self.SecondaryWeapon`
        (:`then`)
        (:`else`
          (set `self.SecondaryWeapon` Weapon))))
    (:`else`
      (set `self.PrimaryWeapon` Weapon)))
  (`|ExecutionSequence`
    (:`then_0`
      (`self.CheckUnEquipedWeapon`
        (:`Is Valid`
          (`self.EquipWeapon` null))))
    (:`then_1`
      (bind _returnvalue (`self.CheckUnEquipedWeapon`)
        (:`Is Valid`
          (`self.Un Equipweapon` _returnvalue))))))

(fn `Un Equipweapon`
  (params (Weapon :type "/Game/FastCampus_TPS/Blueprints/Items/Guns/BP_Gun Object Reference"))
  (`self.K2_AttachToComponent` Weapon (`self.Mesh`) "RifleHolsterSocket" "SnapToTarget" "SnapToTarget" "SnapToTarget" true))

(fn `UserConstructionScript`)