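; BP_Vehicl_Suv is a drivable SUV pawn that the player can enter and exit in a third-person shooter.
; Axis and handbrake inputs drive the VehicleMovement component and controller look.
; Interaction range events toggle custom depth on the mesh, and interacting hides the character, disables its capsule collision and possesses the SUV.
; ExitVehicle restores both, repossesses the stored character and teleports it to a fixed world-space offset from the vehicle.
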(event `InputAxis|MoveForward`
  (params (AxisValue :type "Float (single-precision)"))
  (`WheeledVehicleMovementComponent.SetThrottleInput` (`self.VehicleMovement`) AxisValue))

(event `InputAxis|MoveRight`
  (params (AxisValue :type "Float (single-precision)"))
  (`WheeledVehicleMovementComponent.SetSteeringInput` (`self.VehicleMovement`) AxisValue))

(event `InputAxis|LookUp`
  (params (AxisValue :type "Float (single-precision)"))
  (`self.AddControllerPitchInput` AxisValue))

(event `InputAxis|Turn`
  (params (AxisValue :type "Float (single-precision)"))
  (`self.AddControllerYawInput` AxisValue))

(event `InputAction|HandBreak`
  (params (Key :type "Key Structure"))
  (:`Pressed`
    (`WheeledVehicleMovementComponent.SetHandbrakeInput` (`self.VehicleMovement`) true))
  (:`Released`
    (`WheeledVehicleMovementComponent.SetHandbrakeInput` (`self.VehicleMovement`) false)))

(event `/Game/FastCampus_TPS/Blueprints/Items/BPI_Interaction.OnInteractionRangeEntered`
  (params (InPlayer :type "/Game/FastCampus_TPS/Blueprints/BP_Player_Character Object Reference"))
  (`PrimitiveComponent.SetRenderCustomDepth` (`self.Mesh`) true))

(event `/Game/FastCampus_TPS/Blueprints/Items/BPI_Interaction.OnInteractionRangeExited`
  (`PrimitiveComponent.SetRenderCustomDepth` (`self.Mesh`) false))

(event `/Game/FastCampus_TPS/Blueprints/Items/BPI_Interaction.OnInteracted`
  (params (InPlayer :type "/Game/FastCampus_TPS/Blueprints/BP_Player_Character Object Reference"))
  (bind _playercharacter (`self.PlayerCharacter`))
  (set `self.PlayerCharacter` InPlayer)
  (`PrimitiveComponent.SetRenderCustomDepth` (`self.Mesh`) false)
  (`PrimitiveComponent.SetCollisionEnabled` (`Character.CapsuleComponent` _playercharacter) "NoCollision")
  (`Controller.Possess` (`self.GetController` _playercharacter) self)
  (`SceneComponent.SetVisibility` (`Character.Mesh` (`self.PlayerCharacter`)) false true))

(event `InputAction|ExitVehicle`
  (params (Key :type "Key Structure"))
  (bind _playercharacter (`self.PlayerCharacter`))
  (:`Pressed`
    (bind _playercharacter_2 (`self.PlayerCharacter`)
      (:`then`
        (`PrimitiveComponent.SetCollisionEnabled` (`Character.CapsuleComponent` _playercharacter_2) "QueryAndPhysics")
        (`Controller.Possess` (`self.GetController`) _playercharacter)
        (`self.K2_SetActorLocation` _playercharacter (+ (`self.K2_GetActorLocation`) (100.0 -200.0 100.0)) false true)
        (`SceneComponent.SetVisibility` (`Actor.RootComponent` _playercharacter) true true))
      (:`else`))))

(fn `UserConstructionScript`)